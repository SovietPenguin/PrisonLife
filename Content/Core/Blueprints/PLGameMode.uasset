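; PLGameMode is a game mode Blueprint that runs the game's day-night clock.
; Each tick it advances TimeInSeconds by delta time scaled by TimeMultiplier, wraps at 24 hours, and pitches the directional light to match before refreshing the sky sphere's sun direction.
; It then splits the time into hours, minutes and seconds.
; SetTime and GetTime expose the clock, with SetTime wrapping negative values back from midnight.
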(event EventTick
  (params (DeltaSeconds :type Float%20%28single-precision%29))
  (Utilities|MovetheSunandSet"TimeinSeconds" DeltaSeconds
    (:Out
      (Utilities|CalculateTime))))

(fn ConstructionScript)

(fn SetTime
  (params (New%20time%20in%20seconds :type Float%20%28single-precision%29))
  (if (>= New%20time%20in%20seconds 0.0)
    (Variables|Time|SetTime%20in%20seconds New%20time%20in%20seconds)
    (else
      (Variables|Time|SetTime%20in%20seconds (+ 8.64e+04 New%20time%20in%20seconds)))))

(fn GetTime
  (return (Variables|Time|GetTime%20in%20seconds)))